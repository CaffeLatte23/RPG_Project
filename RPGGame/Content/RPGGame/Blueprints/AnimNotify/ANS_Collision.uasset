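; Anim notify state that opens and closes the melee hit window on an RPG character's current weapon during an animation.
; On notify begin it casts the mesh owner to RPGCharacterBase and, if a weapon is held, calls CollisionAble on it.
; On notify end it calls CollisionDisable on that character's current weapon, so the notify's span on the timeline sets when the weapon's collision is active.
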(fn ReceivedNotifyBegin
  (params (MeshComp :type Skeletal%20Mesh%20Component%20Object%20Reference) (Animation :type Anim%20Sequence%20Base%20Object%20Reference) (TotalDuration :type Float%20%28single-precision%29))
  (bind _asrpgcharacter_base (Utilities|Casting|CastToRPGCharacterBase (Components|GetOwner MeshComp)))
  (if (!= (Variables|/Script/RPGGame.RPGCharacterBase|GetCurrentWeapon _asrpgcharacter_base) 0)
    (Class|RPGWeaponBase|CollisionAble (Variables|/Script/RPGGame.RPGCharacterBase|GetCurrentWeapon _asrpgcharacter_base))
    (return false)))

(fn ReceivedNotifyEnd
  (params (MeshComp :type Skeletal%20Mesh%20Component%20Object%20Reference) (Animation :type Anim%20Sequence%20Base%20Object%20Reference))
  (bind _asrpgcharacter_base (Utilities|Casting|CastToRPGCharacterBase (Components|GetOwner MeshComp)))
  (if (!= (Variables|/Script/RPGGame.RPGCharacterBase|GetCurrentWeapon _asrpgcharacter_base) 0)
    (Class|RPGWeaponBase|CollisionDisable (Variables|/Script/RPGGame.RPGCharacterBase|GetCurrentWeapon _asrpgcharacter_base))
    (return false)))