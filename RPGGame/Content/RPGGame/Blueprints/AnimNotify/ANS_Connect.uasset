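; Anim notify state that marks the combo input window inside the player character's attack montage.
; On begin, it casts the owner to RPGPlayerCharacter, enables the combo period and sets JumpSection to the notify's SectionName.
; On end, it closes the window, clears the attack flag and resets JumpSection to the first combo section.
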(fn ReceivedNotifyBegin
  (params (MeshComp :type Skeletal%20Mesh%20Component%20Object%20Reference) (Animation :type Anim%20Sequence%20Base%20Object%20Reference) (TotalDuration :type Float%20%28single-precision%29))
  (bind _asrpgplayer_character (Utilities|Casting|CastToRPGPlayerCharacter (Components|GetOwner MeshComp)))
  (Variables|/Script/RPGGame.RPGPlayerCharacter|SetbEnableComboPeriod _asrpgplayer_character true)
  (Variables|/Script/RPGGame.RPGPlayerCharacter|SetJumpSection _asrpgplayer_character (Variables|Default|GetSectionName))
  (return false))

(fn ReceivedNotifyEnd
  (params (MeshComp :type Skeletal%20Mesh%20Component%20Object%20Reference) (Animation :type Anim%20Sequence%20Base%20Object%20Reference))
  (bind _asrpgplayer_character (Utilities|Casting|CastToRPGPlayerCharacter (Components|GetOwner MeshComp)))
  (Variables|/Script/RPGGame.RPGPlayerCharacter|SetbEnableComboPeriod _asrpgplayer_character false)
  (Variables|/Script/RPGGame.RPGCharacterBase|SetbIsAttack _asrpgplayer_character false)
  (Variables|/Script/RPGGame.RPGPlayerCharacter|SetJumpSection _asrpgplayer_character "Combo1")
  (return false))