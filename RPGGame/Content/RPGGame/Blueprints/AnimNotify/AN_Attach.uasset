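; AN_Attach is an animation notify that attaches something on an RPG character at a configurable socket and passes along a combat state change.
; It casts the mesh owner to RPGCharacterBase and calls Attach with the notify's socket name and combat values.
; Before attaching, player characters moving at a max walk speed above sprint threshold have their sprint ended.
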(fn ReceivedNotify
  (params (MeshComp :type Skeletal%20Mesh%20Component%20Object%20Reference) (Animation :type Anim%20Sequence%20Base%20Object%20Reference))
  (bind _asrpgcharacter_base (Utilities|Casting|CastToRPGCharacterBase (Components|GetOwner MeshComp)))
  (if (and (> (Variables|/Script/Engine.CharacterMovementComponent|GetMaxWalkSpeed (Variables|/Script/Engine.Character|GetCharacterMovement _asrpgcharacter_base)) 6e+02) (Utilities|IsValid (.AsRPGPlayer%20Character (Utilities|Casting|CastToRPGPlayerCharacter _asrpgcharacter_base))))
    (Class|RPGPlayerCharacter|EndSprint (.AsRPGPlayer%20Character (Utilities|Casting|CastToRPGPlayerCharacter _asrpgcharacter_base))))
  (Default|Attach _asrpgcharacter_base (Variables|Default|GetScoketName) (Variables|Default|GetCombat))
  (return false))