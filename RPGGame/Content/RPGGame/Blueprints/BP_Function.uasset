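; Global helper functions for the RPG game that give quick access to its core Blueprint objects and a world camera shake.
; Getters fetch the player controller, game mode, player character and game instance, cast to their RPG Blueprint types, always using player index 0.
; GetInventoryComp reads the inventory component from the player character.
; ShakeCamera plays a positional shake with radius and falloff, resolving world context through the player's camera manager.
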(fn GetPlayerControllerBP
  (bind _asbp_rpgplayer_controller (Utilities|Casting|CastToBP_RPGPlayerController (Game|GetPlayerController 0))
    (:then
      _)
    (:CastFailed
      _))
  (return _asbp_rpgplayer_controller))

(fn GetGameModeBP
  (bind _asbp_rpggame_mode (Utilities|Casting|CastToBP_RPGGameMode (Game|GetGameMode))
    (:then
      _)
    (:CastFailed
      _))
  (return _asbp_rpggame_mode))

(fn GetPlayerCharacterBP
  (bind _asbp_player (Utilities|Casting|CastToBP_Player (Game|GetPlayerCharacter 0)))
  (return _asbp_player))

(fn GetGameInstanceBP
  (bind _asbp_rpggame_instance (Utilities|Casting|CastToBP_RPGGameInstance (Game|GetGameInstance)))
  (return _asbp_rpggame_instance))

(fn ShakeCamera
  (params (CameraShake%20Class :type Camera%20Shake%20Class%20Reference) (Epicenter :type Vector) (InnerRadius :type Float%20%28single-precision%29) (OuterRadius :type Float%20%28single-precision%29) (FallOff :type Float%20%28single-precision%29))
  (Camera|PlayWorldCameraShake (Game|GetPlayerCameraManager (CallFunction|GetPlayerCharacterBP)) CameraShake%20Class Epicenter InnerRadius OuterRadius FallOff))

(fn GetInventoryComp
  (return (Variables|/Script/RPGGame.RPGPlayerCharacter|GetInventoryComp (CallFunction|GetPlayerCharacterBP))))