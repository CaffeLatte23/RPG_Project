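; RPG game instance Blueprint that loads, applies and persists global options through the "GlobalOptions" save slot.
; GetGlobalSetting returns the stored options, creating and saving a default save object if none exists; only the load branch caches the object.
; SetGlobalSetting updates the HUD's Sousa widget visibility and the game mode's BGM volume, then writes the new options through that cached save object.
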(fn GetGlobalSetting
  (bind _returnvalue (SaveGame|DoesSaveGameExist "GlobalOptions"))
  (if _returnvalue
    (bind _returnvalue_2 (SaveGame|LoadGamefromSlot "GlobalOptions"))
    (bind _asglobal_options_save_game (Utilities|Casting|CastToGlobalOptionsSaveGame _returnvalue_2))
    (Variables|Default|SetNewVar_0 _asglobal_options_save_game)
    (return (Variables|/Game/RPGGame/Blueprints/Other/SaveGame/GlobalOptionsSaveGame.GlobalOptionsSaveGame_C|GetGlobalOptions _asglobal_options_save_game))
    (else
      (bind _returnvalue_3 (SaveGame|CreateSaveGameObject "/Game/RPGGame/Blueprints/Other/SaveGame/GlobalOptionsSaveGame.GlobalOptionsSaveGame_C"))
      (SaveGame|SaveGametoSlot _returnvalue_3 "GlobalOptions")
      (return (Variables|/Game/RPGGame/Blueprints/Other/SaveGame/GlobalOptionsSaveGame.GlobalOptionsSaveGame_C|GetGlobalOptions _returnvalue_3)))))

(fn SetGlobalSetting
  (params (NewOptions :type Global%20Option%20Structure))
  (bind _output_get (LocalVariables|SetNew%20Global%20Options NewOptions))
  (Utilities|FlowControl|Sequence
    (:then_0
      (bind _ashud (Utilities|Casting|CastToHUD (Variables|/Script/RPGGame.RPGPlayerControllerBase|GetHUD (CallFunction|GetPlayerControllerBP))))
      (if (Utilities|IsValid (Variables|/Game/RPGGame/Blueprints/Widgets/HUD.HUD_C|GetWB_Sousa _ashud))
        (Default|UpdateVisibility (Variables|/Game/RPGGame/Blueprints/Widgets/HUD.HUD_C|GetWB_Sousa _ashud) (.sousa_visibility (LocalVariables|GetNew%20Global%20Options)))))
    (:then_1
      (Variables|/Game/RPGGame/Blueprints/BP_RPGGameMode.BP_RPGGameMode_C|SetBGMVolume (CallFunction|GetGameModeBP) (.mainbgmvolume _output_get))
      (Variables|/Game/RPGGame/Blueprints/Other/SaveGame/GlobalOptionsSaveGame.GlobalOptionsSaveGame_C|SetGlobalOptions (Variables|Default|GetNewVar_0) (LocalVariables|GetNew%20Global%20Options))
      (SaveGame|SaveGametoSlot (Variables|Default|GetNewVar_0) "GlobalOptions"))))