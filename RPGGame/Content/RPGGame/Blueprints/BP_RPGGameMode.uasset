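; RPG game mode that shows a floor-start widget for the current floor shortly after BeginPlay and handles fight music switching.
; ChangeMusic alternates between starting and ending the fight music via FlipFlop.
; Timelines drive BGMComp volume, flip its InFight sound parameter on finishing, then reverse, using FirstLoop to stop repeats.
; The code that spawns GameMusic_Cue and assigns BGMComp is disconnected and never runs.
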(event Custom|StartFight
  (bind _bgm_comp (Variables|Default|GetBGM%20Comp))
  ;[1 1 1] Sound Loop
  (bind _music_volume (Timeline|Timeline_0 PlayFromStart)
    (:Update
      (Audio|Components|Audio|SetVolumeMultiplier _bgm_comp _music_volume :!class /Script/Engine.AudioComponent))
    (:Finished
      (if (Variables|Default|GetFirstLoop)
        (Effects|Components|ParticleSystem|SetBoolParameter _bgm_comp "InFight" true)
        (Variables|Default|SetFirstLoop false)
        (Timeline|Timeline_0 Reverse)
        (else
          (Variables|Default|SetFirstLoop true))))))

(event Custom|CustomEvent_0
  ;[1 1 1] Sound Loop
  (bind _music_volume (Timeline|MusicVolume%20Timeline Play)
    (:Update
      (Audio|Components|Audio|SetVolumeMultiplier (Variables|Default|GetBGM%20Comp) _music_volume :!class /Script/Engine.AudioComponent))
    (:Finished
      (if (Variables|Default|GetFirstLoop)
        (Effects|Components|ParticleSystem|SetBoolParameter (Variables|Default|GetBGM%20Comp) "InFight" false)
        (Variables|Default|SetFirstLoop false)
        (Timeline|MusicVolume%20Timeline Reverse)
        (else
          (Variables|Default|SetFirstLoop true))))))

(event EventBeginPlay
  ;[1 1 1] BeginPlay Logic
  (|CallParentFunction)
  (Utilities|FlowControl|Delay 0.01)
  (bind _returnvalue (UserInterface|CreateWidget "/Game/RPGGame/Blueprints/Widgets/WB_FloorStart.WB_FloorStart_C" 0 (Variables|Default|GetFloorNum)))
  (UserInterface|Viewport|AddtoViewport _returnvalue 0))

(event EventChangeMusic
  (params (bIsConnect :type Boolean))
  ;[1 1 1] Sound Loop
  (Utilities|FlowControl|FlipFlop
    (:A
      (CallFunction|StartFight))
    (:B
      (CallFunction|CustomEvent0))))

(fn ConstructionScript)