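; Player controller for the RPG that owns the player's UI: HUD, menus, boss health bar, level-up and game-over screens.
; On first possession it binds to inventory and level-up events, applies camera rate settings and creates weapons.
; Inventory load creates the HUD, and item changes refresh its icons.
; The menu toggle pauses the game, ducks BGM, picks pause or full menu by fight state, and recreates changed weapons on close.
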(event Custom|Inventory%20Load
  ;[0.2033 0.8498 1] Binding Event
  (CallFunction|CreateHUD))

(event Custom|Slotted%20Item%20Changed
  (params (ItemSlot :type RPG%20Item%20Slot%20Structure) (Item :type RPG%20Item%20Object%20Reference))
  ;[0.2033 0.8498 1] Binding Event
  (Class|RPGUIInterface|UpdateIcons(Message) (Variables|Default|GetHUD))
  (Variables|Default|SetWeaponChange (== (.ItemType (Utilities|Struct|BreakRPGItemSlot ItemSlot)) "Weapon")))

(event Custom|OnInventoryChanged
  (params (bAdded :type Boolean) (Item :type RPG%20Item%20Object%20Reference))
  ;[0.2033 0.8498 1] Binding Event
  (Class|RPGUIInterface|UpdateIcons(Message) (Variables|Default|GetHUD)))

(event Custom|Notify%20LevelUP
  (params (NewLv :type Integer))
  ;[0.2033 0.8498 1] Binding Event
  (bind _returnvalue (UserInterface|CreateWidget "/Game/RPGGame/Blueprints/Widgets/WB_LevelUp.WB_LevelUp_C" 0 NewLv))
  (UserInterface|Viewport|AddtoViewport _returnvalue 0))

(event EventPossess
  (params (PossessedPawn :type Pawn%20Object%20Reference))
  (Utilities|FlowControl|DoOnce false
    (:Completed
      (bind _asbp_player (Utilities|Casting|CastToBP_Player PossessedPawn))
      (bind _output_get (Variables|Default|SetPlayerCharacter _asbp_player))
      (Utilities|FlowControl|Sequence
        (:then_0
          ;[0.3545 1 0.3058] Custumize Binding
          (EventDispatchers|BindEventtoOnInventoryLoadedBP (Variables|/Script/RPGGame.RPGPlayerCharacter|GetInventoryComp _output_get) (EventDispatchers|CreateEvent :!event Custom|Inventory%20Load))
          (EventDispatchers|AssignOnSlottedItemChangedBP (Variables|/Script/RPGGame.RPGPlayerCharacter|GetInventoryComp _output_get) (EventDispatchers|CreateEvent :!event Custom|Slotted%20Item%20Changed))
          (EventDispatchers|BindEventtoOnInventoryItemChangedBP (Variables|/Script/RPGGame.RPGPlayerCharacter|GetInventoryComp _output_get) (EventDispatchers|CreateEvent :!event Custom|OnInventoryChanged))
          (EventDispatchers|AssignOnLevelUp (CallFunction|GetPlayerCharacterBP) (EventDispatchers|CreateEvent :!event Custom|Notify%20LevelUP)))
        (:then_1
          ;[1 1 1] PlayerSetting
          (bind _globaloptions (Default|GetGlobalSetting (CallFunction|GetGameInstanceBP)))
          (Variables|/Script/RPGGame.RPGPlayerCharacter|SetBaseLookUpRate (Variables|Default|GetPlayerCharacter) (.cameralookuprate _globaloptions))
          (Variables|/Script/RPGGame.RPGPlayerCharacter|SetBaseTurnRate (Variables|Default|GetPlayerCharacter) (.cameraturnrate _globaloptions))
          (Class|RPGUIInterface|UpdateHP(Message) (Variables|Default|GetHUD) 1.0)
          (Utilities|FlowControl|Delay 0.2)
          (Class|RPGPlayerCharacter|CreateAllWeapons (Variables|Default|GetPlayerCharacter))
          (Input|SetInputModeGameOnly self))))))

(event Input|ActionEvents|InputActionMenu
  (params (Key :type Key%20Structure :default "None"))
  ;[1 1 1] Input
  (:Pressed
    (CallFunction|ShowMenuUI)))

(event Custom|CreateHUD
  ;[1 1 1] HUD作成
  (bind _returnvalue (UserInterface|CreateWidget "/Game/RPGGame/Blueprints/Widgets/HUD.HUD_C" self (Variables|/Script/RPGGame.RPGCharacterBase|GetCharStatus (Variables|Default|GetPlayerCharacter))))
  (bind _output_get (Variables|Default|SetHUD _returnvalue))
  (UserInterface|Viewport|AddtoViewport _output_get 0))

(event Custom|Show%20MenuUI
  (bind _gamemode (CallFunction|GetGameModeBP))
  (bind _self self)
  (bind _bgm_comp (Variables|/Game/RPGGame/Blueprints/BP_RPGGameMode.BP_RPGGameMode_C|GetBGM%20Comp _gamemode))
  (bind _bgmvolume (Variables|/Game/RPGGame/Blueprints/BP_RPGGameMode.BP_RPGGameMode_C|GetBGMVolume _gamemode))
  ;[1 1 1] Menuの作成削除
  (if (Variables|Default|GetbOpenUI)
    (bind _menuui (Variables|Default|GetMenuUI)
      (:then
        (Class|RPGUIInterface|CloseMenu(Message) _menuui)
        (Utilities|FlowControl|Delay 1.0)
        (Audio|Components|Audio|SetVolumeMultiplier _bgm_comp (* _bgmvolume 1.0) :!class /Script/Engine.AudioComponent)
        (Game|SetGamePaused false)
        (Variables|Default|SetMenuUI 0)
        (Input|SetInputModeGameOnly _self)
        (Variables|Default|SetbShowMouseCursor false)
        (Variables|Default|SetbOpenUI false)
        (Variables|Default|SetbSettingChanged false)
        (if (Variables|Default|GetWeaponChange)
          (Class|RPGPlayerCharacter|CreateAllWeapons (Variables|Default|GetPlayerCharacter))
          (Variables|Default|SetWeaponChange false)))
      (:else))
    (else
      (bind _returnvalue (UserInterface|CreateWidget (select (Variables|Default|GetbOnFight) "/Game/RPGGame/Blueprints/Widgets/WB_PauseMenu.WB_PauseMenu_C" "/Game/RPGGame/Blueprints/Widgets/MainMenu/WB_Menu.WB_Menu_C") self))
      (bind _output_get (Variables|Default|SetMenuUI _returnvalue))
      (UserInterface|Viewport|AddtoViewport _output_get 0)
      (Audio|Components|Audio|SetVolumeMultiplier _bgm_comp (* _bgmvolume 0.3) :!class /Script/Engine.AudioComponent)
      (Game|SetGamePaused true)
      (Input|SetInputModeGameandUI _self (Variables|Default|GetMenuUI) "DoNotLock" true)
      (Variables|Default|SetbShowMouseCursor true)
      (Variables|Default|SetbOpenUI true))))

(event EventUpdateHP
  (params (value :type Float%20%28single-precision%29))
  ;[1 1 1] HPBarの更新
  (Default|BarUpdate (Variables|Default|GetBossHP) value))

(event EventTargetIsBoss
  (params (Actor :type RPG%20Enemy%20Base%20Object%20Reference))
  ;[1 1 1] ボスの通知
  (Utilities|IsValid (Variables|Default|GetBossHP)
    (:Is%20Not%20Valid
      (bind _returnvalue (UserInterface|CreateWidget "/Game/RPGGame/Blueprints/Widgets/WB_BossHP.WB_BossHP_C" self Actor))
      (bind _output_get (Variables|Default|SetBossHP _returnvalue))
      (UserInterface|Viewport|AddtoViewport _output_get 0))))

(event EventBossIsDead
  (params (Actor :type Actor%20Object%20Reference))
  ;[1 1 1] ボスの死亡通知
  (if (== Actor (Variables|/Game/RPGGame/Blueprints/Widgets/WB_BossHP.WB_BossHP_C|GetOwner (Variables|Default|GetBossHP)))
    (Default|OwnerDestroy (Variables|Default|GetBossHP))))

(event EventGameOver
  ;[1 1 1] GameOver
  (CallFunction|WidgetHandle "/Game/RPGGame/Blueprints/Widgets/WB_GameOver.WB_GameOver_C"))

(fn ConstructionScript)

(fn WidgetHandle
  (params (NewParam :type User%20Widget%20Class%20Reference))
  (bind _self self)
  (if (Variables|Default|GetbUIOpen)
    (Widget|RemovefromParent (Variables|Default|GetOpenedUI))
    (Input|SetInputModeGameOnly _self)
    (Variables|Default|SetbShowMouseCursor false)
    (Game|SetGamePaused false)
    (Variables|Default|SetbUIOpen false)
    (else
      (bind _returnvalue (UserInterface|CreateWidget NewParam))
      (bind _output_get (Variables|Default|SetOpenedUI _returnvalue))
      (UserInterface|Viewport|AddtoViewport _output_get 0)
      (Input|SetInputModeUIOnly _self _output_get "DoNotLock")
      (Variables|Default|SetbUIOpen true)
      (Game|SetGamePaused true)
      (Variables|Default|SetbShowMouseCursor true))))