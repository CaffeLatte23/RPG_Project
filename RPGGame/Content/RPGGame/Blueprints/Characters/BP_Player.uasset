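; BP_Player is the RPG player character Blueprint, containing an event that rushes the player toward its combat target.
; CloseToTarget picks the locked-on target or PreTarget and acts only if it is valid and over a distance threshold.
; It freezes mesh animation while a timeline repeatedly steps the actor along the look-at direction with swept teleports, scaled by clamped horizontal distance and curve value.
; Animation speed is restored when the timeline finishes.
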(event Custom|CloseToTarget
  (params (NewParam :type Anim%20Montage%20Object%20Reference))
  (bind _returnvalue (Transformation|GetActorLocation))
  (bind _pretarget (Variables|Default|GetPreTarget))
  (bind _blockedontarget (Variables|Default|GetbLockedOnTarget))
  (bind _targetlockactor (Variables|Default|GetTargetLockActor))
  (bind _returnvalue_2 (select _blockedontarget _targetlockactor _pretarget))
  (bind _asactor (Utilities|Casting|CastToActor _returnvalue_2))
  (bind _returnvalue_3 (Transformation|GetActorLocation _asactor))
  (if (and (> (Transformation|GetDistanceTo self _asactor) 2e+02) (Utilities|IsValid _returnvalue_2))
    (Variables|/Script/Engine.SkeletalMeshComponent|SetGlobalAnimRateScale (Variables|Character|GetMesh) 0.0)
    (bind _newtrack_1 (Timeline|Timeline_2 PlayFromStart)
      (:Update
        (Transformation|SetActorLocation (+ (* (Math|Vector|GetForwardVector (Math|Rotator|FindLookatRotation _returnvalue _returnvalue_3)) (* (Math|Float|Clamp(Float) (Math|Vector|VectorLengthXY (- _returnvalue _returnvalue_3)) 5e+01 2e+03) _newtrack_1)) _returnvalue) true true))
      (:Finished
        (Variables|/Script/Engine.SkeletalMeshComponent|SetGlobalAnimRateScale (Variables|Character|GetMesh) 1.0)))))

(event Input|KeyboardEvents|Z
  (params (Key :type Key%20Structure :default "None")))

(fn ConstructionScript)