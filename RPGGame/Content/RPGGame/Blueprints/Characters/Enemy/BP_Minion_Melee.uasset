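; BP_Minion_Melee is a melee enemy minion Blueprint that, as written, only handles floating damage text.
; On capsule overlap it creates a WB_FloatText with a fixed damage value and places it in the viewport at the other actor's projected screen position, without applying damage.
; An unconnected chain holds an alternative world-space widget component version near the current weapon, alongside debug print and line-trace events.
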(event OnComponentBeginOverlap(CapsuleComponent)
  (params (OverlappedComponent :type Primitive%20Component%20Object%20Reference) (OtherActor :type Actor%20Object%20Reference) (OtherComp :type Primitive%20Component%20Object%20Reference) (OtherBodyIndex :type Integer) (bFromSweep :type Boolean) (SweepResult :type Hit%20Result%20Structure%20%28by%20ref%29))
  (bind _returnvalue (UserInterface|CreateWidget "/Game/RPGGame/Blueprints/Widgets/WB_FloatText.WB_FloatText_C" (Game|GetPlayerController 0) 2e+01 0))
  (UserInterface|Viewport|AddtoViewport _returnvalue 0)
  (Class|UserWidget|SetPositioninViewport _returnvalue (.ScreenPosition (Class|GameplayStatics|ProjectWorldtoScreen (Game|GetPlayerController 0) (Transformation|GetActorLocation OtherActor) true)) true))

(event Custom|CustomEvent_0
  (params (NewParam :type Actor%20Object%20Reference))
  ;[1 1 1] 被りで破壊されることへの課題解決
  (Collision|LineTraceByChannel (Transformation|GetActorLocation) (Transformation|GetActorLocation NewParam) "TraceTypeQuery1" false 0 "ForDuration"))

(event Custom|CustomEvent_2
  (params (OverlappedComponent :type Primitive%20Component%20Object%20Reference) (OtherActor :type Actor%20Object%20Reference) (OtherComp :type Primitive%20Component%20Object%20Reference) (OtherBodyIndex :type Integer) (bFromSweep :type Boolean) (SweepResult :type Hit%20Result%20Structure%20%28by%20ref%29))
  ;[1 1 1] 被りで破壊されることへの課題解決
  (Development|PrintString (Utilities|GetDisplayName OtherActor)))

(event Custom|CustomEvent_1
  (params (Component :type Actor%20Component%20Object%20Reference))
  (Development|PrintString (Utilities|GetDisplayName Component)))

(fn ConstructionScript)