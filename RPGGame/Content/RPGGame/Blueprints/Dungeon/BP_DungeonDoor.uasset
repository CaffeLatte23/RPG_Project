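; BP_DungeonDoor is a two-panel sliding dungeon door that opens automatically for the player character.
; When a player enters the Box trigger and DoorLock is off, the DoorAnim timeline slides DoorL and DoorR in opposite directions along X with sweeping.
; Leaving the trigger reverses the timeline to close the door, without checking the lock.
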(event OnComponentBeginOverlap(Box)
  (params (OverlappedComponent :type Primitive%20Component%20Object%20Reference) (OtherActor :type Actor%20Object%20Reference) (OtherComp :type Primitive%20Component%20Object%20Reference) (OtherBodyIndex :type Integer) (bFromSweep :type Boolean) (SweepResult :type Hit%20Result%20Structure%20%28by%20ref%29))
  (bind _asrpgplayer_character (Utilities|Casting|CastToRPGPlayerCharacter OtherActor))
  (Utilities|IsValid _asrpgplayer_character
    (:Is%20Valid
      (if (not (Variables|Default|GetbDoorLock))
        (bind _newtrack_0 (Timeline|Door%20Anim Play)
          (:Update
            (Transformation|SetRelativeLocation (Variables|Default|GetDoorL) (Math|Vector|MakeVector (* _newtrack_0 (Variables|Default|GetNewVar_0)) 0.0 0.0) true false)
            (Transformation|SetRelativeLocation (Variables|Default|GetDoorR) (Math|Vector|MakeVector (* (* _newtrack_0 (Variables|Default|GetNewVar_0)) -1.0) 0.0 0.0) true false)))))))

(event OnComponentEndOverlap(Box)
  (params (OverlappedComponent :type Primitive%20Component%20Object%20Reference) (OtherActor :type Actor%20Object%20Reference) (OtherComp :type Primitive%20Component%20Object%20Reference) (OtherBodyIndex :type Integer))
  (bind _asrpgplayer_character (Utilities|Casting|CastToRPGPlayerCharacter OtherActor))
  (Utilities|IsValid _asrpgplayer_character
    (:Is%20Valid
      (bind _newtrack_0 (Timeline|Door%20Anim Reverse)
        (:Update
          (Transformation|SetRelativeLocation (Variables|Default|GetDoorL) (Math|Vector|MakeVector (* _newtrack_0 (Variables|Default|GetNewVar_0)) 0.0 0.0) true false)
          (Transformation|SetRelativeLocation (Variables|Default|GetDoorR) (Math|Vector|MakeVector (* (* _newtrack_0 (Variables|Default|GetNewVar_0)) -1.0) 0.0 0.0) true false))))))

(fn ConstructionScript)