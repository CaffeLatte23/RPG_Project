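; BP_CameraVolume is a box trigger that sets the camera boom collision test on an overlapping RPGPlayerCharacter.
; Entering the box enables DoCollisionTest.
; Exiting polls every BP_CameraVolume for overlap with the player and, if none is found, also sets DoCollisionTest to true, so nothing here disables it.
; The OtherVolumeOverlapped flag accumulates with OR and is never reset in the graph.
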(event OnComponentBeginOverlap(Box)
  (params (OverlappedComponent :type Primitive%20Component%20Object%20Reference) (OtherActor :type Actor%20Object%20Reference) (OtherComp :type Primitive%20Component%20Object%20Reference) (OtherBodyIndex :type Integer) (bFromSweep :type Boolean) (SweepResult :type Hit%20Result%20Structure%20%28by%20ref%29))
  (bind _asrpgplayer_character (Utilities|Casting|CastToRPGPlayerCharacter OtherActor))
  (Variables|/Script/Engine.SpringArmComponent|SetbDoCollisionTest (Variables|/Script/RPGGame.RPGPlayerCharacter|GetCameraBoom _asrpgplayer_character) true))

(event OnComponentEndOverlap(Box)
  (params (OverlappedComponent :type Primitive%20Component%20Object%20Reference) (OtherActor :type Actor%20Object%20Reference) (OtherComp :type Primitive%20Component%20Object%20Reference) (OtherBodyIndex :type Integer))
  (bind _asrpgplayer_character (Utilities|Casting|CastToRPGPlayerCharacter OtherActor))
  (bind _outactors (Actor|GetAllActorsOfClass "BP_CameraVolume_C"))
  (for _array_element _outactors
    (Variables|Default|SetOtherVolumeOverlapped (or (Collision|IsOverlappingActor (Variables|BP_CameraVolume_C|GetBox _array_element) _asrpgplayer_character :!class /Script/Engine.PrimitiveComponent) (Variables|Default|GetOtherVolumeOverlapped))))
  (if (not (Variables|Default|GetOtherVolumeOverlapped))
    (bind _asrpgplayer_character_2 (Utilities|Casting|CastToRPGPlayerCharacter _asrpgplayer_character))
    (Variables|/Script/Engine.SpringArmComponent|SetbDoCollisionTest (Variables|/Script/RPGGame.RPGPlayerCharacter|GetCameraBoom _asrpgplayer_character_2) true)))

(fn ConstructionScript)