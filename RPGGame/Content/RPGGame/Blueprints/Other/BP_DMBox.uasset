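; Breakable box actor that has a chance to drop a random item after a weapon breaks it.
; The first hit from an RPGWeaponBase stores the box's location, disables physics simulation on the Destructible, narrows its collision and starts a five-second lifespan.
; On destruction, a weighted 40% roll may spawn a random class from the item array slightly above the stored location.
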(event OnComponentHit(Destructible)
  (params (HitComponent :type Primitive%20Component%20Object%20Reference) (OtherActor :type Actor%20Object%20Reference) (OtherComp :type Primitive%20Component%20Object%20Reference) (NormalImpulse :type Vector :default "0, 0, 0") (Hit :type Hit%20Result%20Structure%20%28by%20ref%29))
  (bind _destructible (Variables|Default|GetDestructible))
  ;[1 1 1] HitEvent
  (Utilities|Casting|CastToRPGWeaponBase OtherActor)
  (Utilities|FlowControl|DoOnce false
    (:Completed
      (Variables|Default|SetNewVar_0 (Transformation|GetActorLocation))
      (Physics|SetSimulatePhysics _destructible false)
      (Collision|SetCollisionEnabled _destructible "PhysicsOnly")
      (Collision|SetCollisionResponsetoChannel _destructible "ECC_WorldDynamic" "ECR_Ignore")
      (Actor|SetLifeSpan 5.0))))

(event Custom|DestoryEvent
  (params (DestroyedActor :type Actor%20Object%20Reference))
  (bind _newvar_0 (Variables|Default|GetNewVar_0))
  (bind _spawniemclass (Variables|Default|GetSpawnIemClass))
  (bind (_x _y _z) (Math|Vector|BreakVector _newvar_0))
  ;[1 1 1] Destroy
  (if (Math|Random|RandomBoolwithWeight 0.4)
    (Game|SpawnActorfromClass (Utilities|Array|Get(acopy) _spawniemclass (Math|Random|RandomIntegerinRange 0 (- (Utilities|Array|Length _spawniemclass) 1))) (Math|Transform|MakeTransform (Math|Vector|MakeVector _x _y (+ _z 1e+02)) (Transformation|GetActorRotation)) "Undefined" 0 0)))

(event EventBeginPlay
  ;[1 1 1] Beginplay
  (Game|BindEventtoOnDestroyed (EventDispatchers|CreateEvent :!event Custom|DestoryEvent)))

(fn ConstructionScript)