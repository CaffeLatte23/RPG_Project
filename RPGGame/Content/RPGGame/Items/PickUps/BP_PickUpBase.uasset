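; BP_PickUpBase is a world item pickup with a mesh, a colored point light and a detail widget.
; On begin play it fills the widget from ItemType, and DetailCollision overlaps show or hide it as the player enters or leaves.
; The AnimationCollection event hides the widget, then uses a timeline to shrink the mesh and pull it into the collecting player before destroying the actor.
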(event OnComponentBeginOverlap(DetailCollision)
  (params (OverlappedComponent :type Primitive%20Component%20Object%20Reference) (OtherActor :type Actor%20Object%20Reference) (OtherComp :type Primitive%20Component%20Object%20Reference) (OtherBodyIndex :type Integer) (bFromSweep :type Boolean) (SweepResult :type Hit%20Result%20Structure%20%28by%20ref%29))
  (if (.bSuccess (Utilities|Casting|CastToBP_Player OtherActor))
    (Development|SetHiddeninGame (Variables|Default|GetItemDetail) false false)))

(event OnComponentEndOverlap(DetailCollision)
  (params (OverlappedComponent :type Primitive%20Component%20Object%20Reference) (OtherActor :type Actor%20Object%20Reference) (OtherComp :type Primitive%20Component%20Object%20Reference) (OtherBodyIndex :type Integer))
  (if (.bSuccess (Utilities|Casting|CastToBP_Player OtherActor))
    (Development|SetHiddeninGame (Variables|Default|GetItemDetail) true false)))

(event EventBeginPlay
  (bind _aswb_item_pick_up (Utilities|Casting|CastToWB_Item_PickUp (UserInterface|GetUserWidgetObject (Variables|Default|GetItemDetail))))
  (Default|RefreshItem _aswb_item_pick_up (Variables|Default|GetItemType)))

(event EventAnimationCollection
  (bind _itemmesh (Variables|Default|GetItemMesh))
  ;[1 1 1] Collecting Animation
  (Development|SetHiddeninGame (Variables|Default|GetItemDetail) true false)
  (Variables|Default|SetMeshWorldLocation (Transformation|GetWorldLocation (Variables|Default|GetItemMesh)))
  (bind _alpha (Timeline|Animate Play)
    (:Update
      (Transformation|SetRelativeScale3D _itemmesh (Math|Vector|Lerp(Vector) (Transformation|GetWorldScale (Variables|Default|GetItemMesh)) "0, 0, 0" _alpha))
      (Transformation|SetWorldLocation _itemmesh (Math|Vector|Lerp(Vector) (Variables|Default|GetMeshWorldLocation) (Transformation|GetActorLocation (Variables|Default|GetPlayerCollecting)) _alpha) false true))
    (:Finished
      (Actor|DestroyActor))))

(fn ConstructionScript
  (Rendering|Components|Light|SetLightColor (Variables|Default|GetPointLight) (Variables|Default|GetColor) true))